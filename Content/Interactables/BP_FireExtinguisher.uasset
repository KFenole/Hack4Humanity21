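; VR fire extinguisher actor that motion controllers can pick up, drop and spray.
; Pickup turns off mesh physics, snaps the actor to the grabbing component with a one-hand rotation and records the first hand; Drop detaches and re-enables physics.
; Spray spawns a scaled-down FireSpray actor at the particle spawn point, ignoring its input value.
; Second-hand tracking is only ever cleared, and a delayed projectile spawn is left unconnected.
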(event `/Game/VirtualRealityBP/Blueprints/PickupActorInterface.Pickup`
  (params (AttachTo :type "SceneComponent Object Reference"))
  (if (not (`self.IsFirstHandAttached`))
    (`PrimitiveComponent.SetSimulatePhysics` (`self.StaticMeshComponent`) false)
    (`SceneComponent.K2_AttachToComponent` (`self.K2_GetRootComponent`) AttachTo "None" "SnapToTarget" "SnapToTarget" "KeepWorld" false)
    (`SceneComponent.K2_SetRelativeRotation` (`self.StaticMeshComponent`) (`self.OneHandRotation`) false false)
    (set `self.IsFirstHandAttached` true)
    (set `self.IsSecondHandTrackingActive` false)
    (set `self.FirstHand` AttachTo)))

(event `/Game/VirtualRealityBP/Blueprints/PickupActorInterface.Drop`
  (`PrimitiveComponent.SetSimulatePhysics` (`self.StaticMeshComponent`) true)
  (`self.K2_DetachFromActor` "KeepWorld" "KeepWorld" "KeepWorld")
  (set `self.IsFirstHandAttached` false)
  (set `self.IsSecondHandTrackingActive` false))

(event `self.ReceiveTick`
  (params (DeltaSeconds :type "Float (single-precision)")))

(fn `Spray`
  (params (val :type "Float (double-precision)"))
  (bind _particlespawnpoint (`self.ParticleSpawnPoint`))
  (`|SpawnActorFromClass` "/Game/Interactables/FireSpray.FireSpray_C" (`KismetMathLibrary.MakeTransform` (`SceneComponent.K2_GetComponentLocation` _particlespawnpoint) (`SceneComponent.K2_GetComponentRotation` _particlespawnpoint) (0.1 0.1 0.1)) "Undefined" "OverrideRootScale" null null))

(fn `UserConstructionScript`)